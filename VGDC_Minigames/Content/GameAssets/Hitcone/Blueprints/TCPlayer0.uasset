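; TCPlayer0 is Hitcone's player character, which hunts randomly chosen MannequinAI targets by hitbox collision while Cash drains every second.
; Movement, camera and jump inputs accompany primary-attack swings, animated on the ground or airborne through delay-driven rotation loops.
; Hits match object names against the unique target, paying more during air spins and rerolling until six targets are done.
; Final Cash picks either win camera; any wrong kill triggers the lose camera.
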(event OnComponentHit(HitboxMesh)
  (params (HitComponent :type Primitive%20Component%20Object%20Reference) (OtherActor :type Actor%20Object%20Reference) (OtherComp :type Primitive%20Component%20Object%20Reference) (NormalImpulse :type Vector :default "0, 0, 0") (Hit :type Hit%20Result%20Structure%20%28by%20ref%29))
  (bind _alreadyused (Variables|Default|GetAlreadyUsed))
  ;[1 1 1] Kill People
  (bind _asmannequin_ai (Utilities|Casting|CastToMannequinAI OtherActor)) ; Accesses hit object
  (if (Utilities|Enum|Equal(Enum) (Utilities|GetObjectName _asmannequin_ai) (stale _output_get_2)) ; Wrong Kill if not target
    (if (> (Variables|Default|GetCountAir) 0)
      (Variables|Default|SetCash (+ (Variables|Default|GetCash) 300))
      (else
        (Variables|Default|SetCash (+ (Variables|Default|GetCash) 100))))
    (Audio|PlaySound2D (Utilities|Array|Get(acopy) (Variables|Default|GetDeathSounds) (Math|Random|RandomIntegerinRange 0 13)) 1.0 1.0 0.0 0 0) ; Play random sound
    (Actor|DestroyActor _asmannequin_ai)
    (if (== (Utilities|Array|Length (Variables|Default|GetAlreadyUsed)) 6) ; New target if < 6 killed, end game if 6
      (if (>= (Variables|Default|GetCash) 1200) ; Ending Based on Cash
        ;[1 1 1] Super Win Ending
        (Game|Player|SetViewTargetwithBlend (Game|GetPlayerController 0) (Utilities|ResolveSoftReference (Variables|Default|GetWinCameraActor)) 0.0 "VTBlend_Linear" 0.0 false)
        (Variables|Default|SetEndState 1)
        (else
          ;[1 1 1] Sad Win Ending
          (Game|Player|SetViewTargetwithBlend (Game|GetPlayerController 0) (Utilities|ResolveSoftReference (Variables|Default|GetSadCameraActor)) 0.0 "VTBlend_Linear" 0.0 false)
          (Variables|Default|SetEndState 3)))
      (else
        ;[1 1 1] Target Changing
        (bind _output_get (Variables|Default|SetTargetNum (Math|Random|RandomInteger 11) :!label _label))
        (if (Utilities|Array|ContainsItem _alreadyused _output_get)
          (Development|PrintString "ALREADY DONE!")
          (Utilities|FlowControl|RetriggerableDelay 0.05)
          (goto _label)
          (else
            (bind _output_get_2 (Variables|Default|SetTarget (Utilities|String|Append "MannequinAI" (Utilities|String|ToString(Integer) _output_get))))
            (Variables|Default|SetCurrentPhoto (Utilities|Array|Get(acopy) (Variables|Default|GetVictimPictures) (Variables|Default|GetTargetNum)))
            (Utilities|Array|Add _alreadyused _output_get)
            (Development|PrintString _output_get_2)
            (Development|PrintString (Utilities|String|ToString(Integer) (Utilities|Array|Length _alreadyused)))))))
    (else
      ;[1 1 1] Wrong Kill
      (Game|Player|SetViewTargetwithBlend (Game|GetPlayerController 0) (Utilities|ResolveSoftReference (Variables|Default|GetLoseCameraActor)) 0.0 "VTBlend_Linear" 0.0 false)
      (Variables|Default|SetEndState 2))))

(event EventTick
  (params (DeltaSeconds :type Float%20%28single-precision%29))
  (bind _returnvalue (Utilities|Time|GetRealTimeSeconds))
  ;[1 1 1] Drains Cash per Second
  (if (Math|Boolean|ANDBoolean (>= _returnvalue (+ (Variables|Default|GetLastSecond) 1.0)) (> (Variables|Default|GetCash) 0) (== (Variables|Default|GetEndState) 0))
    (Variables|Default|SetLastSecond _returnvalue)
    (Variables|Default|SetCash (- (Variables|Default|GetCash) 2))))

(event EventBeginPlay
  (bind _alreadyused (Variables|Default|GetAlreadyUsed))
  ;[1 1 1] Target Changing
  (bind _output_get (Variables|Default|SetTargetNum (Math|Random|RandomInteger 11) :!label _label))
  (if (Utilities|Array|ContainsItem _alreadyused _output_get)
    (Development|PrintString "ALREADY DONE!")
    (Utilities|FlowControl|RetriggerableDelay 0.05)
    (goto _label)
    (else
      (bind _output_get_2 (Variables|Default|SetTarget (Utilities|String|Append "MannequinAI" (Utilities|String|ToString(Integer) _output_get))))
      (Variables|Default|SetCurrentPhoto (Utilities|Array|Get(acopy) (Variables|Default|GetVictimPictures) (Variables|Default|GetTargetNum)))
      (Utilities|Array|Add _alreadyused _output_get)
      (Development|PrintString _output_get_2)
      (Development|PrintString (Utilities|String|ToString(Integer) (Utilities|Array|Length _alreadyused))))))

(event Input|ActionEvents|InputActionHitcone_Jump
  (params (Key :type Key%20Structure))
  ;[1 1 1] Movement
  (:Pressed
    (Character|Jump)))

(event Input|ActionEvents|InputActionHitcone_Primary
  (params (Key :type Key%20Structure))
  (bind _tcmesh (Variables|Default|GetTCmesh))
  (bind _count (Variables|Default|GetCount))
  ;[1 1 1] PrimaryGround
  (:Pressed
    (if (not (AI|Components|NavMovement|IsFalling (Variables|Character|GetCharacterMovement))) ; If not falling...
      (if (not (Variables|Default|GetInAnim)) ; If not in animation...
        (if (< _count 16) :!label _label
          (Variables|Default|SetInAnim true)
          (Math|Integer|IncrementInt _count
            (:%20%20
              (Transformation|AddLocalRotation _tcmesh "-6.000000, 0, 0" false false)
              (Utilities|FlowControl|RetriggerableDelay 0.01)
              (goto _label)))
          (else
            (if (> _count 0) :!label _label_2 ; If current frame number is above 0, rotate back up. If at 0, stop animation
              (Math|Integer|DecrementInt _count
                (:%20%20
                  (Transformation|AddLocalRotation _tcmesh "6.000000, 0, 0" false false)
                  (Utilities|FlowControl|RetriggerableDelay 0.01)
                  (goto _label_2)))
              (else
                (Variables|Default|SetInAnim false)))))))))

(event Input|ActionEvents|InputActionHitcone_Primary
  (params (Key :type Key%20Structure))
  (bind _tcmesh (Variables|Default|GetTCmesh))
  ;[1 1 1] PrimaryAir
  (:Pressed
    (if (AI|Components|NavMovement|IsFalling (Variables|Character|GetCharacterMovement)) ; I apologize for lack of documentation. I hope you understand it :)
      (if (not (Variables|Default|GetInAnim))
        (Transformation|SetRelativeRotation _tcmesh "-90.000000, 0, 0" false false)
        (if (< (Variables|Default|GetCountAir) 31) :!label _label
          (Variables|Default|SetInAnim true)
          (Math|Integer|IncrementInt (Variables|Default|GetCountAir)
            (:%20%20
              (Transformation|AddLocalRotation (Variables|Default|GetTCmesh) "0.000000,0.000000,-12.000000" false false)
              (Utilities|FlowControl|RetriggerableDelay 0.01)
              (goto _label)))
          (else
            (Transformation|SetRelativeRotation _tcmesh "0, 0, 0" false false)
            (Variables|Default|SetCountAir 0)
            (Variables|Default|SetInAnim false)))))))

(event Input|AxisEvents|InputAxisHitcone_MoveForward
  (params (AxisValue :type Float%20%28single-precision%29))
  ;[1 1 1] Movement
  (Pawn|Input|AddMovementInput (Math|Vector|GetForwardVector (Math|Rotator|MakeRotator 0.0 0.0 (.Yaw (Math|Rotator|BreakRotator (Pawn|GetControlRotation :!class /Script/Engine.Pawn))))) AxisValue false))

(event Input|AxisEvents|InputAxisHitcone_MoveRight
  (params (AxisValue :type Float%20%28single-precision%29))
  ;[1 1 1] Movement
  (Pawn|Input|AddMovementInput (Math|Vector|GetRightVector (Math|Rotator|MakeRotator 0.0 0.0 (.Yaw (Math|Rotator|BreakRotator (Pawn|GetControlRotation :!class /Script/Engine.Pawn))))) AxisValue false))

(event Input|AxisEvents|InputAxisHitcone_MouseYaw
  (params (AxisValue :type Float%20%28single-precision%29))
  ;[1 1 1] CameraControls
  (Pawn|Input|AddControllerYawInput AxisValue))

(event Input|AxisEvents|InputAxisHitcone_MousePitch
  (params (AxisValue :type Float%20%28single-precision%29))
  ;[1 1 1] CameraControls
  (Pawn|Input|AddControllerPitchInput AxisValue))

(fn ConstructionScript)