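; Base gun Blueprint with hitscan firing and a manual, step-by-step reload mode.
; Shoot, reload and draw events play animations behind an ActionBusy lock timed by delays.
; Each reload press advances a MultiGate animation; the final step refills the magazine or adds one round.
; Shots trace from the player camera on Visibility, looping randomly spread pellets for shotguns, applying damage and drawing beams from the muzzle socket.
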(event Custom|Event%20ReloadGun
  ;[1 1 1] EVENT - Reload Gun
  (if (not (Variables|Default|GetActionBusy))
    (Variables|Default|SetActionBusy true)
    (if (Variables|Default|GetIsReloading)
      ;[1 1 1] check if clip is full
      (if (== (Variables|Default|GetCountBulletsInClip) (Variables|Default|GetClipSize))
        (Development|PrintString "clip full")
        ;[1 1 1] cancel/end reloading mode - loaded
        (Components|Animation|PlayAnimation (Variables|Default|GetGunMesh) (Variables|Default|GetAnimReloadEndLoaded) false)
        (Utilities|FlowControl|Delay (Variables|Default|GetReloadInitializeTime))
        (Variables|Default|SetIsReloading false)
        (Development|PrintString "SHOOT MODE")
        (Variables|Default|SetActionBusy false)
        (else
          ;[1 1 1] check which reload step we are in
          (if (<= (Variables|Default|GetCountStepsThroughReload) (Variables|Default|GetStepsInReload))
            (Development|PrintString "Adding 1 to reload step")
            (Math|Integer|IncrementInt (Variables|Default|GetCountStepsThroughReload)
              (:%20%20
                ;[1 1 1] going through the reload steps - Determining which animation to play
                (Utilities|FlowControl|MultiGate false false -1
                  (:Out%200
                    (Development|PrintString "Start Reload Step 1")
                    (Components|Animation|PlayAnimation (Variables|Default|GetGunMesh) (Variables|Default|GetAnimReloadStep_0) false))
                  (:Out%201
                    (Development|PrintString "Start Reload Step 2")
                    (Components|Animation|PlayAnimation (Variables|Default|GetGunMesh) (Variables|Default|GetAnimReloadStep_1) false))
                  (:Out%202
                    (Development|PrintString "Start Reload Step 3")
                    (Components|Animation|PlayAnimation (Variables|Default|GetGunMesh) (Variables|Default|GetAnimReloadStep_2) false))
                  (:Out%203
                    (Development|PrintString "Start Reload Step 4")
                    (Components|Animation|PlayAnimation (Variables|Default|GetGunMesh) (Variables|Default|GetAnimReloadStep_3) false))
                  (:Out%204
                    (Development|PrintString "Start Reload Step 5")
                    (Components|Animation|PlayAnimation (Variables|Default|GetGunMesh) (Variables|Default|GetAnimReloadStep_4) false)))
                ;;[1 1 1] Actually Reloading
                (CallFunction|FuncReloadGun)
                (Utilities|FlowControl|Delay (Variables|Default|GetReloadStepTime))
                (Development|PrintString "Reloac step Complete")
                (Development|PrintString (Utilities|String|Append (Utilities|String|ToString(Integer) (Variables|Default|GetCountBulletsInClip)) " Bullets In Clip"))
                (Variables|Default|SetActionBusy false)))
            (else
              ;;[1 1 1] Failsafe
              (Variables|Default|SetActionBusy false)))))
      (else
        ;[1 1 1] initialize reloading mode
        (Variables|Default|SetIsReloading true)
        (Development|PrintString "ENTERING RELOAD MODE")
        (Components|Animation|PlayAnimation (Variables|Default|GetGunMesh) (Variables|Default|GetAnimReloadInit) false)
        (Utilities|FlowControl|Delay (Variables|Default|GetReloadInitializeTime))
        (Development|PrintString "RELOAD MODE")
        (Variables|Default|SetActionBusy false)))))

(event Custom|Event%20ShootGun
  (bind _player_cam (Variables|Default|Getplayer_cam))
  (bind _returnvalue (Transformation|GetSocketLocation _player_cam "None"))
  (bind _returnvalue_2 (Transformation|GetWorldRotation _player_cam))
  (bind _returnvalue_3 (Math|Vector|GetForwardVector _returnvalue_2))
  ;[1 1 1] EVENT - Shoot Gun
  (if (not (Variables|Default|GetActionBusy))
    (Variables|Default|SetActionBusy true)
    ;[1 1 1] Check if we are in Reloading Mode
    (if (Variables|Default|GetIsReloading)
      (Development|PrintString "EXITING RELOAD MODE")
      ;[1 1 1] check if clip is full
      (if (== (Variables|Default|GetCountBulletsInClip) (Variables|Default|GetClipSize))
        (Development|PrintString "CLIP FUL")
        ;[1 1 1] cancel/end reloading mode - not loaded
        (Components|Animation|PlayAnimation (Variables|Default|GetGunMesh) (Variables|Default|GetAnimReloadEndLoaded) false)
        (Utilities|FlowControl|Delay (Variables|Default|GetReloadInitializeTime))
        (Variables|Default|SetIsReloading false)
        (Development|PrintString "SHOOT MODE")
        (Variables|Default|SetActionBusy false)
        (else
          ;[1 1 1] check if we are still in reload steps
          (if (<= (Variables|Default|GetCountStepsThroughReload) (Variables|Default|GetStepsInReload))
            (Variables|Default|SetActionBusy false) ; deny reload cancel
            (else
              ;[1 1 1] cancel/end reloading mode - loaded
              (Components|Animation|PlayAnimation (Variables|Default|GetGunMesh) (Variables|Default|GetAnimReloadEndLoaded) false)
              (Utilities|FlowControl|Delay (Variables|Default|GetReloadInitializeTime))
              (Variables|Default|SetIsReloading false)
              (Development|PrintString "SHOOT MODE")
              (Variables|Default|SetActionBusy false)))))
      (else
        ;[1 1 1] check if there is any ammo in the gun
        (if (> (Variables|Default|GetCountBulletsInClip) 0)
          ;[1 1 1] All Checks Passed - Let's Shoot the Gun
          ;;[1 1 1] Check if we are shooting the last bullet
          (if (== (Variables|Default|GetCountBulletsInClip) 1)
            (Components|Animation|PlayAnimation (Variables|Default|GetGunMesh) (Variables|Default|GetAnimFireLast) false)
            ;;[1 1 1] Workaround to prevent reloading until the animation finishes
            (CallFunction|FuncShootGun _returnvalue _returnvalue_3)
            (Utilities|FlowControl|Delay (Variables|/Script/Engine.AnimSequenceBase|GetSequenceLength (Variables|Default|GetAnimFireLast)))
            (else
              (Components|Animation|PlayAnimation (Variables|Default|GetGunMesh) (Variables|Default|GetAnimFireOnce) false)
              ;;[1 1 1] Actually Shoot the Gun
              (CallFunction|FuncShootGun _returnvalue _returnvalue_3)
              (Utilities|FlowControl|Delay (Variables|Default|GetFireRate))))
          (Development|PrintString (Utilities|String|Append (Utilities|String|ToString(Integer) (Variables|Default|GetCountBulletsInClip)) " Bullets In Clip"))
          (Variables|Default|SetActionBusy false)
          (else
            ;[1 1 1] Dry Fire
            (if (Variables|Default|GetIsShotgun) ; Workaround to let shotguns dryfire infinitely
              (Components|Animation|PlayAnimation (Variables|Default|GetGunMesh) (Variables|Default|GetAnimFireDry) false :!label _label)
              (elif (Variables|Default|GetAlreadyDryFired)
                _
                (else
                  (goto _label))))
            (Utilities|FlowControl|Delay 0.2)
            (Variables|Default|SetAlreadyDryFired true) ; This really only applies to the pistol animation
            (Variables|Default|SetActionBusy false)))))))

(event Custom|Event%20DrawWeapon
  ;[1 1 1] EVENT - Draw Weapon Animation
  (Variables|Default|SetActionBusy true)
  (Components|Animation|PlayAnimation (Variables|Default|GetGunMesh) (Variables|Default|GetAnimWeaponDraw) false)
  (Utilities|FlowControl|Delay (Variables|Default|GetWeaponDrawTime))
  (Variables|Default|SetIsReloading false) ; workaround since it has to be a public variable thats changeable  by child classes
  (Variables|Default|SetActionBusy false))

(event Custom|Event%20ResetReloadGate
  ;[1 1 1] going through the reload steps - Determining which animation to play
  (Variables|Default|SetCountStepsThroughReload 0)
  (Utilities|FlowControl|MultiGate false false -1) ; enters at Reset
)

(event EventBeginPlay
  ;[1 1 1] Event Begin Play
  (Variables|Default|SetCountBulletsInClip (Variables|Default|GetClipSize))
  (Variables|Default|SetCountStepsThroughReload 0)
  ;;[1 1 1] setting the camera variable from the player camera
  (Variables|Default|Setplayer_cam (Variables|/Script/Engine.Actor|GetRootComponent (Game|GetPlayerCameraManager 0)))
  (Variables|Default|SetIsReloading false) ; workaround since it has to be a public variable thats changeable  by child classes
)

(event Collision|EventActorBeginOverlap
  (params (OtherActor :type Actor%20Object%20Reference)))

(event EventTick
  (params (DeltaSeconds :type Float%20%28single-precision%29)))

(fn ConstructionScript)

(fn FuncShootGun
  (params (StartLocation :type Vector) (StartRotationVector :type Vector))
  (bind _bulletspread (Variables|Default|GetBulletSpread))
  (bind (_x _y _z) (Math|Vector|BreakVector StartRotationVector))
  (bind _returnvalue (* _bulletspread 1.0))
  (bind _returnvalue_2 (* _returnvalue -1.0))
  ;[1 1 1] shoot gun - hitscan
  ;;[1 1 1] setup local variables
  (bind _output_get (LocalVariables|SetTrace%20Start%20Location StartLocation))
  (bind _output_get_2 (LocalVariables|SetTraceStartRotation StartRotationVector))
  (LocalVariables|SetTraceEndLocation (+ _output_get (* _output_get_2 (Variables|Default|GetMaxBulletDistance))))
  ;;[1 1 1] check if we have a shotgun
  (if (Variables|Default|GetIsShotgun)
    ;;[1 1 1] Shotgun Ammo spread loop and shooting
    ;;;[1 1 1] Loop Until there are no more pellets in the round
    (bind _output_get_3 (LocalVariables|SetCountPellets (Variables|Default|GetSG_pellets)))
    (while (> _output_get_3 0)
      (CallFunction|FuncRayTraceShot (LocalVariables|GetTrace%20Start%20Location) (LocalVariables|GetTraceEndLocation))
      ;;;[1 1 1] 1 Trace done - Subtract 1 pellet
      (Math|Integer|DecrementInt (LocalVariables|GetCountPellets)
        (:%20%20
          ;;;[1 1 1] Set new TraceEnd from random rotation
          (LocalVariables|SetTraceEndLocation (+ StartLocation (* (Math|Vector|RotateVector StartRotationVector (Math|Rotator|MakeRotator (+ _x (Math|Random|RandomFloatinRange _returnvalue_2 _returnvalue)) (+ _y (Math|Random|RandomFloatinRange _returnvalue_2 _returnvalue)) (+ _z (Math|Random|RandomFloatinRange _returnvalue_2 _returnvalue)))) (Variables|Default|GetMaxBulletDistance))))
          (Development|PrintString "fired pellet"))))
    (Development|PrintString "Shotgun done")
    (else
      ;;[1 1 1] Fire a Single Shot
      (CallFunction|FuncRayTraceShot (LocalVariables|GetTrace%20Start%20Location) (LocalVariables|GetTraceEndLocation))))
  ;;[1 1 1] Remove 1 ammo
  (Math|Integer|DecrementInt (Variables|Default|GetCountBulletsInClip)
    (:%20%20
      (Development|PrintString "1 shot fired"))))

(fn FuncReloadGun
  ;[1 1 1] Checking if we are done with reload steps
  (if (== (Variables|Default|GetCountStepsThroughReload) (Variables|Default|GetStepsInReload))
    (Development|PrintString "Steps completed. Reloading Gun")
    (CallFunction|EventResetReloadGate)
    (Variables|Default|SetAlreadyDryFired false)
    (if (Variables|Default|GetHasMagazine)
      ;[1 1 1] Reload entire magazine
      (Variables|Default|SetCountBulletsInClip (Variables|Default|GetClipSize))
      (else
        ;[1 1 1] Reload one bullet
        (if (< (Variables|Default|GetCountBulletsInClip) (Variables|Default|GetClipSize))
          (Math|Integer|IncrementInt (Variables|Default|GetCountBulletsInClip)))))
    (else
      (Development|PrintString "Reload Steps Not complete"))))

(fn FuncRayTraceShot
  (params (TraceStartLocation :type Vector) (TraceEndLocation :type Vector))
  (bind _gunmesh (Variables|Default|GetGunMesh))
  (bind _returnvalue (Transformation|GetSocketLocation _gunmesh "muzzleSocket"))
  (bind (_outhit _returnvalue_2) (Collision|LineTraceByChannel TraceStartLocation TraceEndLocation "TraceTypeQuery1" false (Utilities|Array|MakeArray (Game|GetPlayerCharacter 0)) "None")) ; The visibility channel means theres no hitboxes, and literally checks what's visible
  (if _returnvalue_2 ; Splits outcome based on whether or not the trace hit something
    ;[1 1 1] If trace hits something
    (bind _returnvalue_3 (AddComponent|AddParticleSystemComponent false))
    (Class|ParticleSystemComponent|SetBeamSourcePoint _returnvalue_3 0 _returnvalue)
    (Class|ParticleSystemComponent|SetBeamTargetPoint _returnvalue_3 0 (.Location (Collision|BreakHitResult _outhit)))
    (Effects|SpawnEmitteratLocation "/Game/StarterContent/Particles/P_Explosion.P_Explosion" (.Location (Collision|BreakHitResult _outhit)))
    (Game|Damage|ApplyDamage (.HitActor (Collision|BreakHitResult _outhit)) (Variables|Default|GetDamage) 0 0)
    (else
      ;[1 1 1] If trace misses and hits nothing
      (bind _returnvalue_4 (AddComponent|AddParticleSystemComponent false))
      (Class|ParticleSystemComponent|SetBeamSourcePoint _returnvalue_4 0 _returnvalue)
      (Class|ParticleSystemComponent|SetBeamTargetPoint _returnvalue_4 0 TraceEndLocation))))