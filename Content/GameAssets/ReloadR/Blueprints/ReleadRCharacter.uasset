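; Player character for a shooter, handling movement, mouse look, jump, crouch and weapon input.
; BeginPlay spawns four guns attached hidden to the hand and shows Secondary1; number keys swap guns by visibility, blocked during reloads.
; Shooting and reloading are delegated to the equipped gun.
; Damage, or the V key, enables a post-process effect and sets AboutToDie; old projectile and jump-gravity logic is mostly disconnected.
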(event EventBeginPlay
  ;[1 1 1] Event BeginPlay
  (CallFunction|SpawnWeapons)
  ;;[1 1 1] setting default/initial weapon to secondary1
  (bind _output_get (Variables|Default|SetEquippedGun (Variables|Default|GetSecondary1)))
  (Rendering|SetVisibility (Variables|/Game/GameAssets/ReloadR/Blueprints/BP_gun_base.BP_gun_base_C|GetDefaultSceneRoot _output_get) true true))

(event Collision|EventActorBeginOverlap
  (params (OtherActor :type Actor%20Object%20Reference)))

(event EventTick
  (params (DeltaSeconds :type Float%20%28single-precision%29)))

(event EventOnLanded
  (params (Hit :type Hit%20Result%20Structure%20%28by%20ref%29))
  ;[1 1 1] [DEFUNCT] Attempt at custom jump arc
  (Variables|/Script/Engine.CharacterMovementComponent|SetGravityScale (Variables|Character|GetCharacterMovement) 2.0))

(event Game|Damage|EventAnyDamage
  (params (Damage :type Float%20%28single-precision%29) (DamageType :type Damage%20Type%20Object%20Reference) (InstigatedBy :type Controller%20Object%20Reference) (DamageCauser :type Actor%20Object%20Reference))
  ;[1 1 1] Post Process and Damage
  (Development|PrintString "YOU WERE HIT")
  (Variables|/Script/Engine.PostProcessComponent|SetBlendWeight (Variables|Default|GetCharacterPostProcess) 1.0)
  (Variables|Default|SetAboutToDie true))

(event Input|AxisEvents|InputAxisHitcone_MoveForward
  (params (AxisValue :type Float%20%28single-precision%29))
  ;[1 1 1] Movement
  (Pawn|Input|AddMovementInput (Math|Vector|GetForwardVector (Math|Rotator|MakeRotator 0.0 0.0 (.Yaw (Math|Rotator|BreakRotator (Pawn|GetControlRotation :!class /Script/Engine.Pawn))))) AxisValue false))

(event Input|AxisEvents|InputAxisHitcone_MoveRight
  (params (AxisValue :type Float%20%28single-precision%29))
  ;[1 1 1] Movement
  (Pawn|Input|AddMovementInput (Math|Vector|GetRightVector (Math|Rotator|MakeRotator 0.0 0.0 (.Yaw (Math|Rotator|BreakRotator (Pawn|GetControlRotation :!class /Script/Engine.Pawn))))) AxisValue false))

(event Input|MouseEvents|MouseX
  (params (AxisValue :type Float%20%28single-precision%29))
  ;[1 1 1] CameraControls
  (Pawn|Input|AddControllerYawInput (* AxisValue (Variables|Default|GetCameraSensetivityVar))))

(event Input|MouseEvents|MouseY
  (params (AxisValue :type Float%20%28single-precision%29))
  ;[1 1 1] CameraControls
  (Pawn|Input|AddControllerPitchInput (* (* AxisValue (Variables|Default|GetCameraSensetivityVar)) -1.0)))

(event Input|KeyboardEvents|R
  (params (Key :type Key%20Structure))
  ;[1 1 1] reloading - Event withing BP_gun_base
  (:Pressed
    (Default|EventReloadGun (Variables|Default|GetEquippedGun))))

(event Input|KeyboardEvents|SpaceBar
  (params (Key :type Key%20Structure))
  ;[1 1 1] Jumping
  (:Pressed
    (Character|Jump)))

(event Input|KeyboardEvents|1
  (params (Key :type Key%20Structure))
  ;[1 1 1] Weapon Switching
  (:Pressed
    (CallFunction|SwitchWeapon (Variables|Default|GetPrimary1) (Variables|Default|GetEquippedGun))))

(event Input|KeyboardEvents|LeftShift
  (params (Key :type Key%20Structure))
  ;[1 1 1] crouching
  (:Pressed
    (Character|Crouch))
  (:Released
    (Character|UnCrouch)))

(event Input|KeyboardEvents|V
  (params (Key :type Key%20Structure))
  ;[1 1 1] Post Process and Damage
  (:Pressed
    (Development|PrintString "YOU WERE HIT")
    (Variables|/Script/Engine.PostProcessComponent|SetBlendWeight (Variables|Default|GetCharacterPostProcess) 1.0)
    (Variables|Default|SetAboutToDie true)))

(event Input|KeyboardEvents|2
  (params (Key :type Key%20Structure))
  ;[1 1 1] Weapon Switching
  (:Pressed
    (CallFunction|SwitchWeapon (Variables|Default|GetSecondary1) (Variables|Default|GetEquippedGun))))

(event Input|MouseEvents|LeftMouseButton
  (params (Key :type Key%20Structure))
  ;[1 1 1] [DEFUNCT] shoot gun - projectile
)

(event Input|KeyboardEvents|3
  (params (Key :type Key%20Structure))
  ;[1 1 1] Weapon Switching
  (:Pressed
    (CallFunction|SwitchWeapon (Variables|Default|GetPrimary2) (Variables|Default|GetEquippedGun))))

(event Input|MouseEvents|LeftMouseButton
  (params (Key :type Key%20Structure))
  ;[1 1 1] shoot gun - event within BP_gun_base
  (:Pressed
    (Default|EventShootGun (Variables|Default|GetEquippedGun))))

(event Input|KeyboardEvents|4
  (params (Key :type Key%20Structure))
  ;[1 1 1] Weapon Switching
  (:Pressed
    (CallFunction|SwitchWeapon (Variables|Default|GetSecondary2) (Variables|Default|GetEquippedGun))))

(fn ConstructionScript)

(fn SwitchWeapon
  (params (NewWeapon :type BP%20Gun%20Base%20Object%20Reference) (CurrentWeapon :type BP%20Gun%20Base%20Object%20Reference))
  ;[1 1 1] Check if the gun is currently being reloaded
  (if (not (Variables|/Game/GameAssets/ReloadR/Blueprints/BP_gun_base.BP_gun_base_C|GetIsReloading (Variables|Default|GetEquippedGun)))
    ;[1 1 1] check if new weapon is already equipped
    (if (not (== NewWeapon CurrentWeapon))
      ;[1 1 1] Disable Current Weapon
      (Rendering|SetVisibility (Variables|/Game/GameAssets/ReloadR/Blueprints/BP_gun_base.BP_gun_base_C|GetDefaultSceneRoot CurrentWeapon) false true)
      ;[1 1 1] Enable New Weapon, Set it as the new equipped weapon, and Trigger Draw Weapon Animation
      (bind _output_get (Variables|Default|SetEquippedGun NewWeapon))
      (Rendering|SetVisibility (Variables|/Game/GameAssets/ReloadR/Blueprints/BP_gun_base.BP_gun_base_C|GetDefaultSceneRoot _output_get) true true)
      (Default|EventDrawWeapon (Variables|Default|GetEquippedGun)))))

(fn SpawnWeapons
  ;[1 1 1] Rinse and repeat for each weapon
  (Utilities|FlowControl|Sequence
    (:then_0
      ;[1 1 1] Spawn weapon BP and give it a variable name
      (bind _returnvalue (Game|SpawnActorfromClass "/Game/GameAssets/ReloadR/Blueprints/BP_gun001.BP_gun001_C" (Math|Transform|MakeTransform "0, 0, 0" "0, 0, 0" "1,1,1") "AlwaysSpawn" 0 0))
      (bind _output_get (Variables|Default|SetSecondary1 _returnvalue))
      ;[1 1 1] Attach the spawned weapon to the hand location
      (Transformation|AttachComponentToComponent _output_get (Variables|Default|GetRWeaponAttachment) "None" "SnapToTarget" "SnapToTarget" "KeepRelative" true)
      ;[1 1 1] Disable the weapon so it doesn't show
      (Rendering|SetVisibility (Variables|/Game/GameAssets/ReloadR/Blueprints/BP_gun_base.BP_gun_base_C|GetDefaultSceneRoot (Variables|Default|GetSecondary1)) false true))
    (:then_1
      (bind _returnvalue_2 (Game|SpawnActorfromClass "/Game/GameAssets/ReloadR/Blueprints/BP_gun002.BP_gun002_C" (Math|Transform|MakeTransform "0, 0, 0" "0, 0, 0" "1,1,1") "AlwaysSpawn" 0 0))
      (bind _output_get_2 (Variables|Default|SetSecondary2 _returnvalue_2))
      (Transformation|AttachComponentToComponent _output_get_2 (Variables|Default|GetRWeaponAttachment) "None" "SnapToTarget" "SnapToTarget" "KeepRelative" true)
      (Rendering|SetVisibility (Variables|/Game/GameAssets/ReloadR/Blueprints/BP_gun_base.BP_gun_base_C|GetDefaultSceneRoot (Variables|Default|GetSecondary2)) false true))
    (:then_2
      (bind _returnvalue_3 (Game|SpawnActorfromClass "/Game/GameAssets/ReloadR/Blueprints/BP_gun003.BP_gun003_C" (Math|Transform|MakeTransform "0, 0, 0" "0, 0, 0" "1,1,1") "AlwaysSpawn" 0 0))
      (bind _output_get_3 (Variables|Default|SetPrimary1 _returnvalue_3))
      (Transformation|AttachComponentToComponent _output_get_3 (Variables|Default|GetRWeaponAttachment) "None" "SnapToTarget" "SnapToTarget" "KeepRelative" true)
      (Rendering|SetVisibility (Variables|/Game/GameAssets/ReloadR/Blueprints/BP_gun_base.BP_gun_base_C|GetDefaultSceneRoot (Variables|Default|GetPrimary1)) false true))
    (:then_3
      (bind _returnvalue_4 (Game|SpawnActorfromClass "/Game/GameAssets/ReloadR/Blueprints/BP_gun004.BP_gun004_C" (Math|Transform|MakeTransform "0, 0, 0" "0, 0, 0" "1,1,1") "AlwaysSpawn" 0 0))
      (bind _output_get_4 (Variables|Default|SetPrimary2 _returnvalue_4))
      (Transformation|AttachComponentToComponent _output_get_4 (Variables|Default|GetRWeaponAttachment) "None" "SnapToTarget" "SnapToTarget" "KeepRelative" true)
      (Rendering|SetVisibility (Variables|/Game/GameAssets/ReloadR/Blueprints/BP_gun_base.BP_gun_base_C|GetDefaultSceneRoot (Variables|Default|GetPrimary2)) false true))))