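; AI controller for the ReloadR simple enemy that starts its behavior tree when play begins.
; On BeginPlay it sets up the simple-enemy blackboard and stores the controlled pawn's spawn position as HomeLocation.
; It then runs the simple-enemy behavior tree, printing debug messages for the home vector and tree start.
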(event EventBeginPlay
  (bind _returnvalue (Pawn|GetControlledPawn))
  (bind _returnvalue_2 (Transformation|GetActorLocation _returnvalue))
  (Class|AIController|UseBlackboard "/Game/GameAssets/ReloadR/Blueprints/EnemyAI/BB_reloadR_SimpleEnemy.BB_reloadR_SimpleEnemy")
  (AI|Components|Blackboard|SetValueasVector (AI|GetBlackboard self) (Variables|Default|GetHomeLocation) _returnvalue_2)
  (Development|PrintString (Utilities|String|Append "Home Vector: " (Utilities|String|ToString(Vector) _returnvalue_2)))
  (Development|PrintString "BehaviorTree Running")
  (AI|RunBehaviorTree "/Game/GameAssets/ReloadR/Blueprints/EnemyAI/BT_reloadR_SimpleEnemy.BT_reloadR_SimpleEnemy"))

(event EventTick
  (params (DeltaSeconds :type Float%20%28single-precision%29)))

(fn ConstructionScript)