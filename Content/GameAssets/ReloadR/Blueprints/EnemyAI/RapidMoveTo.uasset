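; RapidMoveTo is a Behavior Tree task that moves the AI-controlled enemy pawn toward the actor stored in the TargetToFollow blackboard key.
; On execute it caches the BP_reloadR_AI_Controller, then runs AIMoveTo with AcceptableRadius, which must stay smaller than AcceptableDistance in EnemyCloseEnough.
; Both success and failure print a debug string and finish the task as failed.
; If the owner cast fails, the task never calls FinishExecute.
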(event EventReceiveExecute
  (params (OwnerActor :type Actor%20Object%20Reference))
  (if (!= (Variables|Default|GetAI_CONTROLLER_Ref) 0)
    _
    (else
      (bind _asbp_reload_r_ai_controller (Utilities|Casting|CastToBP_reloadR_AI_Controller OwnerActor))
      (Variables|Default|SetAI_CONTROLLER_Ref _asbp_reload_r_ai_controller)))
  (AI|AIMoveTo (Pawn|GetControlledPawn (Variables|Default|GetAI_CONTROLLER_Ref)) "0, 0, 0" (AI|BehaviorTree|GetBlackboardValueasActor (Variables|Default|GetTargetToFollow)) (Variables|Default|GetAcceptableRadius) false
    (:OnSuccess
      (Development|PrintString "WISHES TO KILL ENEMY"))
    (:OnFail
      (Development|PrintString "DOOR STUCK")))
  (AI|BehaviorTree|FinishExecute false))