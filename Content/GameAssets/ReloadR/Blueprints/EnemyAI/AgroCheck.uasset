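; Behavior tree service that checks each tick for targets the controlled enemy can see within its aggro distance.
; It caches the AI controller, then sphere-traces around the pawn for the desired object types, ignoring all BP_SimpleEnemy actors.
; Each hit gets a visibility line trace: visible actors set TargetToFollow and TargetLocation, blocked ones clear TargetToFollow.
; The last hit processed decides TargetToFollow, and zero hits leave it unchanged.
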(event EventTick
  (params (OwnerActor :type Actor%20Object%20Reference) (DeltaSeconds :type Float%20%28single-precision%29))
  (bind _targettofollow (Variables|Default|GetTargetToFollow))
  ;[1 1 1] Check if not blank
  (if (!= (Variables|Default|GetAI_CONROLLER_Ref) 0)
    _
    (else
      (bind _asbp_reload_r_ai_controller (Utilities|Casting|CastToBP_reloadR_AI_Controller OwnerActor))
      (Variables|Default|SetAI_CONROLLER_Ref _asbp_reload_r_ai_controller)))
  (bind _outactors (Actor|GetAllActorsOfClass "/Game/GameAssets/ReloadR/Blueprints/BP_SimpleEnemy.BP_SimpleEnemy_C"))
  (Variables|Default|SetMyLocation (Transformation|GetActorLocation (Pawn|GetControlledPawn (Variables|Default|GetAI_CONROLLER_Ref))))
  (bind _outhits (Collision|MultiSphereTraceForObjects (Transformation|GetActorLocation (Pawn|GetControlledPawn (Variables|Default|GetAI_CONROLLER_Ref))) (+ (Transformation|GetActorLocation (Pawn|GetControlledPawn (Variables|Default|GetAI_CONROLLER_Ref))) "0, 0,15.000000") (Variables|Default|GetAgroDistance) (Variables|Default|GetDesiredObjectTypes) false _outactors "None"))
  (bind _array_element (Utilities|Array|ForEachLoopwithBreak _outhits)
    (:LoopBody
      (bind _outhit (Collision|LineTraceByChannel (Variables|Default|GetMyLocation) (Transformation|GetActorLocation (.HitActor (Collision|BreakHitResult _array_element))) "TraceTypeQuery1" false _outactors "None"))
      (if (== (.HitActor (Collision|BreakHitResult _outhit)) (.HitActor (Collision|BreakHitResult _array_element)))
        (Development|PrintString "ENEMY SPOTTED")
        (Class|BTFunctionLibrary|SetBlackboardValueasObject _targettofollow (.HitActor (Collision|BreakHitResult _outhit)))
        (AI|BehaviorTree|SetBlackboardValueasVector (Variables|Default|GetTargetLocation) (Transformation|GetActorLocation (.HitActor (Collision|BreakHitResult _outhit))))
        (else
          (Development|PrintString "Nothing in sight")
          (Class|BTFunctionLibrary|SetBlackboardValueasObject _targettofollow))))))