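; Behavior tree decorator for ReloadR enemy AI that checks how far the controlled pawn is from its follow target.
; It casts the owner to BP_reloadR_AI_Controller and measures the distance to the TargetToFollow blackboard actor.
; Despite the EnemyCloseEnough name, it passes when that distance is at least AcceptableDistance.
; AcceptableDistance is meant to sit slightly above the RapidMoveTo acceptance radius.
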(fn PerformConditionCheck
  (params (OwnerActor :type Actor%20Object%20Reference))
  (bind _asbp_reload_r_ai_controller (Utilities|Casting|CastToBP_reloadR_AI_Controller OwnerActor))
  (Variables|Default|SetAI_CONTROLLER_Ref _asbp_reload_r_ai_controller)
  (return (>= (Math|Vector|VectorLength (- (Transformation|GetActorLocation (AI|BehaviorTree|GetBlackboardValueasActor (Variables|Default|GetTargetToFollow))) (Transformation|GetActorLocation (Pawn|GetControlledPawn (Variables|Default|GetAI_CONTROLLER_Ref))))) (Variables|Default|GetAcceptableDistance))))