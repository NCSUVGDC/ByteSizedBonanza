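; BP_SimpleEnemy is an armed enemy that, on taking any damage, is replaced by a BP_exp_barrel which immediately receives damage, in a Creeper-style death.
; On BeginPlay it spawns a BP_gun001 and snaps it to the hand attachment component.
; The EnemyShoot event forwards firing to that gun.
; Navmesh player tracking via AIMoveTo is marked defunct, and its timer setup is unconnected.
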(event Custom|AI%20TrackPlayer
  ;[1 1 1] [DEFUNCT] Simple Move to the player using navmesh navigation
  (AI|AIMoveTo (Variables|Default|GetVarAIPawn) "0, 0, 0" (Variables|Default|GetVarPlayerChar) 1e+02 false))

(event Custom|Event%20EnemyShoot
  ;[1 1 1] Enemy Shoots the gun
  (Default|EventShootGun (Variables|Default|GetSecondary1)))

(event EventBeginPlay
  ;[1 1 1] Spawn weapon BP and give it a variable name
  (bind _returnvalue (Game|SpawnActorfromClass "/Game/GameAssets/ReloadR/Blueprints/BP_gun001.BP_gun001_C" (Math|Transform|MakeTransform "0, 0, 0" "0, 0, 0" "1,1,1") "AlwaysSpawn" 0 0))
  (bind _output_get (Variables|Default|SetSecondary1 _returnvalue))
  ;[1 1 1] Attach the spawned weapon to the hand location
  (Transformation|AttachComponentToComponent _output_get (Variables|Default|GetRWeaponAttachment) "None" "SnapToTarget" "SnapToTarget" "KeepRelative" true))

(event Collision|EventActorBeginOverlap
  (params (OtherActor :type Actor%20Object%20Reference)))

(event EventTick
  (params (DeltaSeconds :type Float%20%28single-precision%29)))

(event Game|Damage|EventAnyDamage
  (params (Damage :type Float%20%28single-precision%29) (DamageType :type Damage%20Type%20Object%20Reference) (InstigatedBy :type Controller%20Object%20Reference) (DamageCauser :type Actor%20Object%20Reference))
  ;[1 1 1] Creeper, awww man...
  (bind _returnvalue (Game|SpawnActorfromClass "/Game/GameAssets/ReloadR/Blueprints/BP_exp_barrel.BP_exp_barrel_C" (Math|Transform|MakeTransform (Transformation|GetWorldLocation (Variables|Collision|GetCapsuleComponent)) "0, 0, 0" "1,1,1") "Undefined" 0 0))
  (Actor|DestroyActor)
  (Game|Damage|ApplyDamage _returnvalue 1.0 0 0))

(fn ConstructionScript)