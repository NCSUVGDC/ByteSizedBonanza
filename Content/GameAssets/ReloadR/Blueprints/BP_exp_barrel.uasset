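; Exploding barrel that bursts into a shotgun-like spray of damaging line traces when it takes any damage.
; A one-time flag prevents re-triggering before FuncExplode fires the traces from the mesh along its forward vector, randomly rotating each after the first.
; Each trace draws a beam particle, and hits also spawn an explosion emitter and apply damage.
; The barrel then disables collision, hides its mesh and destroys itself after a short delay.
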(event EventBeginPlay)

(event Collision|EventActorBeginOverlap
  (params (OtherActor :type Actor%20Object%20Reference)))

(event EventTick
  (params (DeltaSeconds :type Float%20%28single-precision%29)))

(event Game|Damage|EventAnyDamage
  (params (Damage :type Float%20%28single-precision%29) (DamageType :type Damage%20Type%20Object%20Reference) (InstigatedBy :type Controller%20Object%20Reference) (DamageCauser :type Actor%20Object%20Reference))
  (bind _staticmesh (Variables|Default|GetStaticMesh))
  ;[1 1 1] Prevent Infinite Loop
  (if (not (Variables|Default|GetAlreadyExploded))
    (Variables|Default|SetAlreadyExploded true)
    (CallFunction|FuncExplode (Transformation|GetWorldLocation _staticmesh) (Math|Vector|GetForwardVector (Transformation|GetWorldRotation _staticmesh)))
    (Collision|SetActorEnableCollision false)
    (Rendering|SetVisibility (Variables|Default|GetStaticMesh) false true)
    (Utilities|FlowControl|Delay 3.0)
    (Actor|DestroyActor)))

(fn ConstructionScript)

(fn FuncExplode
  (params (StartLocation :type Vector) (StartRotationVector :type Vector))
  (bind _tracespread (Variables|Default|GetTraceSpread))
  (bind _returnvalue (* _tracespread 1.0))
  (bind _returnvalue_2 (* _returnvalue -1.0))
  ;[1 1 1] setup local variables
  (bind _output_get (LocalVariables|SetTrace%20Start%20Location StartLocation))
  (bind _output_get_2 (LocalVariables|SetTraceStartRotation StartRotationVector))
  (LocalVariables|SetTraceEndLocation (+ _output_get (* _output_get_2 (Variables|Default|GetMaxTraceDistance))))
  ;[1 1 1] Loop Until there are no more pellets in the round
  (bind _output_get_3 (LocalVariables|SetCountPellets (Variables|Default|GetNumTraces)))
  (while (> _output_get_3 0)
    (bind (_outhit _returnvalue_3) (Collision|LineTraceByChannel (LocalVariables|GetTrace%20Start%20Location) (LocalVariables|GetTraceEndLocation) "TraceTypeQuery1" false 0 "None"))
    (if _returnvalue_3 ; Splits outcome based on whether or not the trace hit something
      ;[1 1 1] If trace hits something
      (bind _returnvalue_4 (AddComponent|AddParticleSystemComponent false))
      (Class|ParticleSystemComponent|SetBeamSourcePoint _returnvalue_4 0 (LocalVariables|GetTrace%20Start%20Location))
      (Class|ParticleSystemComponent|SetBeamTargetPoint _returnvalue_4 0 (.Location (Collision|BreakHitResult _outhit)))
      (Effects|SpawnEmitteratLocation "/Game/StarterContent/Particles/P_Explosion.P_Explosion" (.Location (Collision|BreakHitResult _outhit)))
      (Game|Damage|ApplyDamage (.HitActor (Collision|BreakHitResult _outhit)) (Variables|Default|GetDamagePerTrace) 0 0)
      (else
        ;[1 1 1] If trace misses and hits nothing
        (bind _returnvalue_5 (AddComponent|AddParticleSystemComponent false))
        (Class|ParticleSystemComponent|SetBeamSourcePoint _returnvalue_5 0 (LocalVariables|GetTrace%20Start%20Location))
        (Class|ParticleSystemComponent|SetBeamTargetPoint _returnvalue_5 0 (LocalVariables|GetTraceEndLocation))))
    ;[1 1 1] 1 Trace done - Subtract 1 pellet
    (Math|Integer|DecrementInt (LocalVariables|GetCountPellets)
      (:%20%20
        ;[1 1 1] Set new TraceEnd from random rotation
        (LocalVariables|SetTraceEndLocation (+ (LocalVariables|GetTrace%20Start%20Location) (* (Math|Vector|RotateVector (LocalVariables|GetTraceStartRotation) (Math|Rotator|MakeRotator (+ (.X (Math|Vector|BreakVector (LocalVariables|GetTraceStartRotation))) (Math|Random|RandomFloatinRange _returnvalue_2 _returnvalue)) (+ (.Y (Math|Vector|BreakVector (LocalVariables|GetTraceStartRotation))) (Math|Random|RandomFloatinRange _returnvalue_2 _returnvalue)) (+ (.Z (Math|Vector|BreakVector (LocalVariables|GetTraceStartRotation))) (Math|Random|RandomFloatinRange _returnvalue_2 _returnvalue)))) (Variables|Default|GetMaxTraceDistance))))
        (Development|PrintString "fired pellet"))))
  (Development|PrintString "Barrel Exploded Done"))