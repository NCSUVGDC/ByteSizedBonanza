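; Player-controlled golf ball with mouse-orbit camera, axis-driven zoom and a PowerBar widget created at BeginPlay.
; Holding left mouse ramps a capped launch speed; releasing sets the physics sphere's velocity along the camera's yaw.
; While charging, Tick allows launches only when the ball is nearly still and zeroes slow drift.
; Tick also moves the spring arm to just above the sphere each frame.
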(event EventBeginPlay
  (bind _returnvalue (UserInterface|CreateWidget "/Game/GameAssets/InterPlanetaryGolf/PowerBar.PowerBar_C"))
  (UserInterface|Viewport|AddtoViewport _returnvalue 0))

(event EventTick
  (params (DeltaSeconds :type Float%20%28single-precision%29))
  (bind _springarm (Variables|Default|GetSpringArm))
  ;[1 1 1] Monitor status of ball
  (Transformation|SetWorldLocation (Variables|Default|GetSpringArm) (+ (Transformation|GetWorldLocation (Variables|Default|GetSphere)) "0, 0,40.000000") false false)
  (if (Variables|Default|GetisCharging)
    (if (Variables|Default|GetcanLaunch)
      (Variables|Default|SetLaunchSpeed (Math|Float|Min(Float) (+ (* DeltaSeconds 1.5e+03) (Variables|Default|GetLaunchSpeed)) 5e+03)))
    (if (<= (Math|Vector|VectorLength (Transformation|GetComponentVelocity (Variables|Default|GetSphere))) 0.1)
      (Variables|Default|SetcanLaunch true)
      (else
        (Variables|Default|SetcanLaunch false)))
    (if (<= (Math|Vector|VectorLength (Transformation|GetComponentVelocity (Variables|Default|GetSphere))) 18.0)
      (Physics|SetPhysicsLinearVelocity (Variables|Default|GetSphere) "0, 0, 0" false "None")))
  ;;[1 1 1] set camera distance
  (Variables|/Script/Engine.SpringArmComponent|SetTargetArmLength _springarm (+ (* (Class|Actor|GetInputAxisKeyValue) 2e+01) (Variables|/Script/Engine.SpringArmComponent|GetTargetArmLength _springarm))))

(event Input|MouseEvents|MouseY
  (params (AxisValue :type Float%20%28single-precision%29))
  ;[1 1 1] Camera Controls
  (Pawn|Input|AddControllerPitchInput (* AxisValue -1.0)))

(event Input|MouseEvents|MouseX
  (params (AxisValue :type Float%20%28single-precision%29))
  ;[1 1 1] Camera Controls
  (Pawn|Input|AddControllerYawInput AxisValue))

(event Input|MouseEvents|LeftMouseButton
  (params (Key :type Key%20Structure))
  ;[1 1 1] Charge Stroke
  (:Pressed
    (Variables|Default|SetisCharging true))
  (:Released
    ;[1 1 1] Launch Ball
    (if (and (Variables|Default|GetisCharging) (Variables|Default|GetcanLaunch))
      (Physics|SetPhysicsLinearVelocity (Variables|Default|GetSphere) (* (Math|Vector|GetForwardVector (Math|Rotator|MakeRotator 0.0 0.0 (.Yaw (Math|Rotator|BreakRotator (Pawn|GetControlRotation :!class /Script/Engine.Pawn))))) (Variables|Default|GetLaunchSpeed)) false "None")
      (Variables|Default|SetcanLaunch false)
      (Variables|Default|SetLaunchSpeed 0.0)
      (Variables|Default|SetisCharging false)
      (else
        (Variables|Default|SetisCharging false)
        (Variables|Default|SetLaunchSpeed 0.0)))))

(fn ConstructionScript)