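; Convex ramp actor for the interplanetary golf game that redirects the golf ball as it rolls over in either direction.
; Two box triggers record which was hit last in MostRecent, so crossing order reveals the travel direction.
; When the ball reaches one trigger after the other, its Direction is set to a fixed-magnitude vector along the actor's or first box's X axis, signed by travel direction.
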(event OnComponentBeginOverlap(Box)
  (params (OverlappedComponent :type Primitive%20Component%20Object%20Reference) (OtherActor :type Actor%20Object%20Reference) (OtherComp :type Primitive%20Component%20Object%20Reference) (OtherBodyIndex :type Integer) (bFromSweep :type Boolean) (SweepResult :type Hit%20Result%20Structure%20%28by%20ref%29))
  ;[1 1 1] Going forwards on the ramp
  (bind _asgolf_ball_bp (Utilities|Casting|CastToGolfBallBP OtherActor)
    (:then
      _)
    (:CastFailed
      _))
  (if (== (Variables|Default|GetmostRecent) 2)
    (Variables|/Game/GameAssets/InterPlanetaryGolf/Blueprints/GolfBallBP.GolfBallBP_C|Setdirection _asgolf_ball_bp (* (Math|Rotator|GetRotationXVector (Transformation|GetActorRotation)) -30)))
  (Variables|Default|SetmostRecent 1))

(event OnComponentBeginOverlap(Box2)
  (params (OverlappedComponent :type Primitive%20Component%20Object%20Reference) (OtherActor :type Actor%20Object%20Reference) (OtherComp :type Primitive%20Component%20Object%20Reference) (OtherBodyIndex :type Integer) (bFromSweep :type Boolean) (SweepResult :type Hit%20Result%20Structure%20%28by%20ref%29))
  ;[1 1 1] Going backwards on ramp
  (bind _asgolf_ball_bp (Utilities|Casting|CastToGolfBallBP OtherActor)
    (:then
      _)
    (:CastFailed
      _))
  (if (== (Variables|Default|GetmostRecent) 1)
    (Variables|/Game/GameAssets/InterPlanetaryGolf/Blueprints/GolfBallBP.GolfBallBP_C|Setdirection _asgolf_ball_bp (* (Math|Rotator|GetRotationXVector (Transformation|GetWorldRotation (Variables|Default|GetBox))) 30)))
  (Variables|Default|SetmostRecent 2))

(fn ConstructionScript)