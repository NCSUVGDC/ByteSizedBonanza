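; Player-controlled golf ball for InterPlanetaryGolf, with mouse orbit camera, adjustable zoom, power bar and stroke counter.
; Holding left mouse charges capped launch speed; releasing fires along control rotation, counts a stroke and saves the ball's transform and gravity.
; While charging, Tick halts a slow ball and allows launching only at rest.
; Custom gravity adds a Direction vector to velocity every frame without delta-time scaling, switched between six axes by number keys.
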(event EventBeginPlay
  ;[1 1 1] add ui components
  (bind _returnvalue (UserInterface|CreateWidget "/Game/GameAssets/InterPlanetaryGolf/UIComponents/PowerBar.PowerBar_C"))
  (UserInterface|Viewport|AddtoViewport _returnvalue 0)
  (bind _returnvalue_2 (UserInterface|CreateWidget "/Game/GameAssets/InterPlanetaryGolf/UIComponents/StrokeCounter.StrokeCounter_C"))
  (UserInterface|Viewport|AddtoViewport _returnvalue_2 0)
  ;[1 1 1] set initial values
  (Variables|Default|Setdirection "0, 0,-30.000000")
  (Variables|Default|Setstrokes 0))

(event EventTick
  (params (DeltaSeconds :type Float%20%28single-precision%29))
  (bind _springarm (Variables|Default|GetSpringArm))
  (bind _sphere (Variables|Default|GetSphere))
  (bind _direction (Variables|Default|Getdirection))
  ;[1 1 1] Monitor status of ball
  (Transformation|SetWorldLocation (Variables|Default|GetSpringArm) (Transformation|GetWorldLocation (Variables|Default|GetSphere)) false false)
  (if (Variables|Default|GetisCharging)
    (if (Variables|Default|GetcanLaunch)
      (Variables|Default|SetLaunchSpeed (Math|Float|Min(Float) (+ (* DeltaSeconds 1.5e+03) (Variables|Default|GetLaunchSpeed)) 5e+03)))
    (if (<= (Math|Vector|VectorLength (Transformation|GetComponentVelocity (Variables|Default|GetSphere))) 0.1)
      (Variables|Default|SetcanLaunch true)
      (else
        (Variables|Default|SetcanLaunch false)))
    (if (<= (Math|Vector|VectorLength (Transformation|GetComponentVelocity (Variables|Default|GetSphere))) 18.0)
      (Physics|SetPhysicsLinearVelocity (Variables|Default|GetSphere) "0, 0, 0" false "None")))
  ;;[1 1 1] set camera distance
  (Variables|/Script/Engine.SpringArmComponent|SetTargetArmLength _springarm (+ (* (Class|Actor|GetInputAxisKeyValue) 2e+01) (Variables|/Script/Engine.SpringArmComponent|GetTargetArmLength _springarm)))
  ;;[1 1 1] Apply Gravity
  (bind _returnvalue (Physics|GetPhysicsLinearVelocity _sphere "None"))
  (Physics|SetPhysicsLinearVelocity _sphere (+ _returnvalue _direction) false "None")
  (Development|PrintString (Utilities|String|ToString(Vector) _direction)))

(event Input|MouseEvents|MouseY
  (params (AxisValue :type Float%20%28single-precision%29))
  ;[1 1 1] Camera Controls
  (Pawn|Input|AddControllerPitchInput (* AxisValue -1.0)))

(event Input|MouseEvents|MouseX
  (params (AxisValue :type Float%20%28single-precision%29))
  ;[1 1 1] Camera Controls
  (Pawn|Input|AddControllerYawInput AxisValue))

(event Input|MouseEvents|LeftMouseButton
  (params (Key :type Key%20Structure))
  (bind _returnvalue (Pawn|GetControlRotation :!class /Script/Engine.Pawn))
  (bind (_roll _pitch _yaw) (Math|Rotator|BreakRotator _returnvalue))
  ;[1 1 1] Launch Ball
  ;;[1 1 1] Charge Stroke
  (:Pressed
    (Variables|Default|SetisCharging true))
  (:Released
    (if (and (Variables|Default|GetisCharging) (Variables|Default|GetcanLaunch))
      (Physics|SetPhysicsLinearVelocity (Variables|Default|GetSphere) (* (Math|Vector|GetForwardVector (Math|Rotator|MakeRotator _roll _pitch _yaw)) (Variables|Default|GetLaunchSpeed)) false "None")
      ;;[1 1 1] Set variables
      (Variables|Default|SetcanLaunch false)
      (Variables|Default|SetLaunchSpeed 0.0)
      (Variables|Default|SetisCharging false)
      (Math|Integer|IncrementInt (Variables|Default|Getstrokes)
        (:%20%20
          (Variables|Default|SetLastLocation (Transformation|GetWorldLocation (Variables|Default|GetSphere)))
          (Variables|Default|SetLastRotation (Transformation|GetWorldRotation (Variables|Default|GetSphere)))
          (Variables|Default|SetLastDirection (Variables|Default|Getdirection))))
      (else
        (Variables|Default|SetisCharging false)
        (Variables|Default|SetLaunchSpeed 0.0)))))

(event Input|KeyboardEvents|1
  (params (Key :type Key%20Structure))
  ;[1 1 1] control gravity (needs to change)
  (:Pressed
    (Variables|Default|Setdirection "0, 0,40.000000")))

(event Input|KeyboardEvents|2
  (params (Key :type Key%20Structure))
  ;[1 1 1] control gravity (needs to change)
  (:Pressed
    (Variables|Default|Setdirection "0, 0,-40.000000")))

(event Input|KeyboardEvents|3
  (params (Key :type Key%20Structure))
  ;[1 1 1] control gravity (needs to change)
  (:Pressed
    (Variables|Default|Setdirection "40.000000, 0, 0")))

(event Input|KeyboardEvents|4
  (params (Key :type Key%20Structure))
  ;[1 1 1] control gravity (needs to change)
  (:Pressed
    (Variables|Default|Setdirection "-40.000000, 0, 0")))

(event Input|KeyboardEvents|5
  (params (Key :type Key%20Structure))
  ;[1 1 1] control gravity (needs to change)
  (:Pressed
    (Variables|Default|Setdirection "0,-40.000000, 0")))

(event Input|KeyboardEvents|6
  (params (Key :type Key%20Structure))
  ;[1 1 1] control gravity (needs to change)
  (:Pressed
    (Variables|Default|Setdirection "0,40.000000, 0")))

(fn ConstructionScript)