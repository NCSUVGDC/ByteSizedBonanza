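; DeathBox is a boundary volume for the interplanetary golf game that resets the golf ball when it stops overlapping the box.
; On end overlap, it restores the GolfBallBP's last location, rotation and direction, zeroes linear velocity and plays a bonk sound.
; It also plays a one-time mistake voice line per box instance if GameState's GlobalVoice is idle, storing the new audio component there.
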(event OnComponentEndOverlap(Box)
  (params (OverlappedComponent :type Primitive%20Component%20Object%20Reference) (OtherActor :type Actor%20Object%20Reference) (OtherComp :type Primitive%20Component%20Object%20Reference) (OtherBodyIndex :type Integer))
  ;[1 1 1] restore golf ball to state before bad launch
  (bind _asgolf_ball_bp (Utilities|Casting|CastToGolfBallBP OtherActor))
  (Variables|/Game/GameAssets/InterPlanetaryGolf/Blueprints/GolfBallBP.GolfBallBP_C|Setdirection _asgolf_ball_bp (Variables|/Game/GameAssets/InterPlanetaryGolf/Blueprints/GolfBallBP.GolfBallBP_C|GetLastDirection _asgolf_ball_bp))
  (Transformation|SetWorldLocationAndRotation (Variables|/Game/GameAssets/InterPlanetaryGolf/Blueprints/GolfBallBP.GolfBallBP_C|GetSphere _asgolf_ball_bp) (Variables|/Game/GameAssets/InterPlanetaryGolf/Blueprints/GolfBallBP.GolfBallBP_C|GetLastLocation _asgolf_ball_bp) (Variables|/Game/GameAssets/InterPlanetaryGolf/Blueprints/GolfBallBP.GolfBallBP_C|GetLastRotation _asgolf_ball_bp) false false)
  (Physics|SetPhysicsLinearVelocity (Variables|/Game/GameAssets/InterPlanetaryGolf/Blueprints/GolfBallBP.GolfBallBP_C|GetSphere _asgolf_ball_bp) "0, 0, 0" false "None")
  (Audio|PlaySound2D "/Game/GameAssets/InterPlanetaryGolf/Audio/sfx/bonk.bonk" 1.0 1.0 0.0 0 0)
  ;[1 1 1] Logic for playing voice line
  (bind _outactors (Actor|GetAllActorsOfClass "/Game/GameAssets/InterPlanetaryGolf/Blueprints/GameState.GameState_C"))
  ;[1 1 1] Play Death Voice
  (if (and (not (Audio|Components|Audio|IsPlaying (Variables|/Game/GameAssets/InterPlanetaryGolf/Blueprints/GameState.GameState_C|GetGlobalVoice (Utilities|Array|Get(acopy) _outactors)))) (not (Variables|Default|GetHas%20Played%20Death)))
    (bind _outactors_2 (Actor|GetAllActorsOfClass "/Game/GameAssets/InterPlanetaryGolf/Blueprints/GameState.GameState_C"))
    (bind _returnvalue (Audio|SpawnSound2D "/Game/GameAssets/InterPlanetaryGolf/Audio/voices/Mistake.Mistake" 1.0 1.0 0.0 0 false false))
    (Variables|/Game/GameAssets/InterPlanetaryGolf/Blueprints/GameState.GameState_C|SetGlobalVoice (Utilities|Array|Get(acopy) _outactors_2) _returnvalue)
    (Variables|Default|SetHas%20Played%20Death true)))

(event EventBeginPlay)

(event Collision|EventActorBeginOverlap
  (params (OtherActor :type Actor%20Object%20Reference)))

(event EventTick
  (params (DeltaSeconds :type Float%20%28single-precision%29)))

(fn ConstructionScript)