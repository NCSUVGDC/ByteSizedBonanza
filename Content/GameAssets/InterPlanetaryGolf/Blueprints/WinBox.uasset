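; WinBox is the goal trigger in InterPlanetaryGolf that ends play when its Box component is overlapped.
; Any overlap fires it, with no check on the other actor, and stops GlobalMusic and GlobalVoice on the GameState found via GetAllActorsOfClass.
; It then plays the Finish sound, replaces all widgets with the EndScreen, shows the mouse cursor and pauses the game.
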(event OnComponentBeginOverlap(Box)
  (params (OverlappedComponent :type Primitive%20Component%20Object%20Reference) (OtherActor :type Actor%20Object%20Reference) (OtherComp :type Primitive%20Component%20Object%20Reference) (OtherBodyIndex :type Integer) (bFromSweep :type Boolean) (SweepResult :type Hit%20Result%20Structure%20%28by%20ref%29))
  (bind _outactors (Actor|GetAllActorsOfClass "/Game/GameAssets/InterPlanetaryGolf/Blueprints/GameState.GameState_C"))
  (Audio|Components|Audio|Stop (Variables|/Game/GameAssets/InterPlanetaryGolf/Blueprints/GameState.GameState_C|GetGlobalMusic (Utilities|Array|Get(acopy) _outactors)))
  (bind _outactors_2 (Actor|GetAllActorsOfClass "/Game/GameAssets/InterPlanetaryGolf/Blueprints/GameState.GameState_C"))
  (Audio|Components|Audio|Stop (Variables|/Game/GameAssets/InterPlanetaryGolf/Blueprints/GameState.GameState_C|GetGlobalVoice (Utilities|Array|Get(acopy) _outactors_2)))
  (Audio|PlaySound2D "/Game/GameAssets/InterPlanetaryGolf/Audio/voices/Finish.Finish" 1.0 1.0 0.0 0 0)
  (Viewport|RemoveAllWidgets)
  (bind _returnvalue (UserInterface|CreateWidget "/Game/GameAssets/InterPlanetaryGolf/UIComponents/EndScreen.EndScreen_C"))
  (UserInterface|Viewport|AddtoViewport _returnvalue 0)
  (Variables|/Script/Engine.PlayerController|SetbShowMouseCursor (Game|GetPlayerController 0) true)
  (Game|SetGamePaused true))

(event EventBeginPlay)

(event Collision|EventActorBeginOverlap
  (params (OtherActor :type Actor%20Object%20Reference)))

(event EventTick
  (params (DeltaSeconds :type Float%20%28single-precision%29)))

(fn ConstructionScript)